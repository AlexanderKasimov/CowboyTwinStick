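; Boss demon enemy for a 2D Paper2D game that lines up vertically with the player and strikes horizontally.
; Tick drives a state machine: it moves along Z until aligned, then attacks, or charges to the farther side obstacle found by box traces when too close in X.
; Flipbook completion chains attack stages, firing a damaging box trace between them, and finishes death.
; A ZAvoidance obstacle search is defined but never called here.
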(event `self.HandleDeath`
  (params (DeathCause :type "/Game/BP/Enum_DeathCause Enum" :default "NewEnumerator0"))
  (set `self.State` "NewEnumerator4")
  (bind _flipbook (`self.GetAnimation`))
  (`PaperFlipbookComponent.SetFlipbook` (`self.PaperFlipbook`) _flipbook)
  (`PaperFlipbookComponent.SetLooping` (`self.PaperFlipbook`) false)
  (`PaperFlipbookComponent.PlayFromStart` (`self.PaperFlipbook`)))

(event `self.ReceiveTick`
  (params (DeltaSeconds :type "Float (single-precision)"))
  (bind _returnvalue (`GameplayStatics.GetPlayerPawn` 0))
  (bind _returnvalue_2 (`GameplayStatics.GetPlayerPawn` 0))
  (`|ExecutionSequence`
    (:`then_0`
      (`/Engine/EditorBlueprintResources/StandardMacros.IsValid` _returnvalue_2
        (:`Is Valid`
          (if (<= (.x (- (`self.K2_GetActorLocation` _returnvalue_2) (`self.K2_GetActorLocation`))) 0.0)
            (set `self.FacingDirection` "NewEnumerator0")
            (else
              (set `self.FacingDirection` "NewEnumerator1"))))))
    (:`then_1`
      (switch `/Game/BP/Enum_AiStates` (`self.State`)
        (:`NewEnumerator1`
          (`/Engine/EditorBlueprintResources/StandardMacros.IsValid` _returnvalue
            (:`Is Valid`
              (set `self.zReached` (<= (`KismetMathLibrary.Abs` (.z (- (`self.K2_GetActorLocation` _returnvalue) (`self.K2_GetActorLocation`)))) (/ (`self.AttackWidth`) 2.0)))
              (if (not (`self.zReached`))
                (if (> (`KismetMathLibrary.Abs` (.x (- (`self.K2_GetActorLocation` (`GameplayStatics.GetPlayerPawn` 0)) (`self.K2_GetActorLocation`)))) (/ (`self.xSize`) 2.0))
                  (set `self.MovementDirection` (`KismetMathLibrary.Normal` (- (`self.K2_GetActorLocation` (`GameplayStatics.GetPlayerPawn` 0)) (`self.K2_GetActorLocation`))))
                  (`self.K2_SetActorLocation` (+ (`self.K2_GetActorLocation`) (* (`KismetMathLibrary.MakeVector` 0.0 0.0 (.z (`self.MovementDirection`))) (`self.MovementSpeed`))) true)
                  (else
                    (set `self.State` "NewEnumerator2")
                    (bind _chargelocation (`self.GetChargeLocation`))
                    (set `self.AvoidanceCoord` _chargelocation)))
                (else
                  (set `self.State` "NewEnumerator3")
                  (bind _flipbook (`self.GetAnimation`))
                  (`PaperFlipbookComponent.SetFlipbook` (`self.PaperFlipbook`) _flipbook)
                  (`PaperFlipbookComponent.SetLooping` (`self.PaperFlipbook`) false)
                  (`PaperFlipbookComponent.PlayFromStart` (`self.PaperFlipbook`)))))))
        (:`NewEnumerator2`
          (set `self.isAvoided` (<= (`KismetMathLibrary.Abs` (.x (- (`self.AvoidanceCoord`) (`self.K2_GetActorLocation`)))) (/ (`self.xSize`) 2.0)))
          (if (`self.isAvoided`)
            (set `self.State` "NewEnumerator1")
            (else
              (`self.K2_SetActorLocation` (+ (`self.K2_GetActorLocation`) (* (`KismetMathLibrary.Normal` (- (`self.AvoidanceCoord`) (`self.K2_GetActorLocation`))) (`self.ChargeSpeed`))) true))))))
    (:`then_2`
      (switch `/Game/BP/Enum_AiStates` (`self.State`)
        (:`NewEnumerator1`
          _)
        (:`NewEnumerator2`
          _))
      (bind _flipbook_2 (`self.GetAnimation`))
      (`PaperFlipbookComponent.SetFlipbook` (`self.PaperFlipbook`) _flipbook_2)
      (`PaperFlipbookComponent.SetLooping` (`self.PaperFlipbook`) true))))

(event `self.PaperFlipbook.OnFinishedPlaying`
  (switch `/Game/BP/Enum_AiStates` (`self.State`)
    (:`NewEnumerator3`
      (if (or (== (`PaperFlipbookComponent.GetFlipbook` (`self.PaperFlipbook`)) "/Game/Sprites/BossDemon/BossDemonAttackLeft/FB_BossDemonAttackLeft_Begin.FB_BossDemonAttackLeft_Begin") (== (`PaperFlipbookComponent.GetFlipbook` (`self.PaperFlipbook`)) "/Game/Sprites/BossDemon/BossDemonAttackLeft/FB_BossDemonAttackLeft_Begin.FB_BossDemonAttackLeft_Begin"))
        (`|ExecutionSequence`
          (:`then_0`
            (bind _flipbook (`self.GetAnimation`))
            (`PaperFlipbookComponent.SetFlipbook` (`self.PaperFlipbook`) _flipbook)
            (`PaperFlipbookComponent.PlayFromStart` (`self.PaperFlipbook`)))
          (:`then_1`
            (`self.Attack`)))
        (elif (or (== (`PaperFlipbookComponent.GetFlipbook` (`self.PaperFlipbook`)) "/Game/Sprites/BossDemon/BossDemonAttackLeft/FB_BossDemonAttackLeft_End.FB_BossDemonAttackLeft_End") (== (`PaperFlipbookComponent.GetFlipbook` (`self.PaperFlipbook`)) "/Game/Sprites/BossDemon/BossDemonAttackLeft/FB_BossDemonAttackLeft_End.FB_BossDemonAttackLeft_End"))
          (set `self.State` "NewEnumerator1")
          (`PaperFlipbookComponent.PlayFromStart` (`self.PaperFlipbook`)))))
    (:`NewEnumerator4`
      (`parent.HandleDeath` "NewEnumerator0"))))

(fn `Attack`
  (bind _outhit (`KismetSystemLibrary.BoxTraceSingle` :`Start` (+ (`self.K2_GetActorLocation`) (* (`KismetMathLibrary.MakeVector` (.x (`KismetMathLibrary.Normal` (- (`self.K2_GetActorLocation` (`GameplayStatics.GetPlayerPawn` 0)) (`self.K2_GetActorLocation`))))) 32.0)) :`End` (+ (`self.K2_GetActorLocation`) (* (`KismetMathLibrary.MakeVector` (.x (`KismetMathLibrary.Normal` (- (`self.K2_GetActorLocation` (`GameplayStatics.GetPlayerPawn` 0)) (`self.K2_GetActorLocation`))))) 320.0)) :`HalfSize` (`KismetMathLibrary.Conv_DoubleToVector` (`self.AttackWidth`)) :`TraceChannel` "TraceTypeQuery1" :`bTraceComplex` true :`DrawDebugType` "ForDuration"))
  (bind (_bblockinghit _binitialoverlap _time _distance _location _impactpoint _normal _impactnormal _physmat _hitactor) (`GameplayStatics.BreakHitResult` _outhit))
  (if _bblockinghit
    (bind _returnvalue (`self.GetComponentByClass` _hitactor "/Game/BP/BP_BaseHealthComponent.BP_BaseHealthComponent_C"))
    (`/Engine/EditorBlueprintResources/StandardMacros.IsValid` _returnvalue
      (:`Is Valid`
        (message `/Game/BP/IDamagable.HandleDamage` _returnvalue (`self.AttackDamage`) "NewEnumerator3")))))

(fn `GetAnimation`
  (returns (Flipbook :type "PaperFlipbook Object Reference"))
  (bind _returnvalue (`PaperFlipbookComponent.GetFlipbook` (`self.PaperFlipbook`)))
  ;[1 1 1] Candidat To BaseClass
  (switch `/Game/BP/Enum_AiStates` (`self.State`)
    (:`NewEnumerator5`
      (return (select `/Game/BP/Enum_AIFacingDirection` (`self.FacingDirection`) :`NewEnumerator0` "/Game/Sprites/BossDemon/BossDemonIdle/FB_BossDemonIdle.FB_BossDemonIdle" :`NewEnumerator1` "/Game/Sprites/BossDemon/BossDemonIdle/FB_BossDemonIdle.FB_BossDemonIdle" :!type "PaperFlipbook Object Reference")))
    (:`NewEnumerator1`
      (if (> (`KismetMathLibrary.VSize` (`self.MovementDirection`)) 0.0)
        (return (select `/Game/BP/Enum_AIFacingDirection` (`self.FacingDirection`) :`NewEnumerator0` "/Game/Sprites/BossDemon/BossDemonWalk/FB_BossDemonWalk.FB_BossDemonWalk" :`NewEnumerator1` "/Game/Sprites/BossDemon/BossDemonWalk/FB_BossDemonWalk.FB_BossDemonWalk" :!type "PaperFlipbook Object Reference"))
        (else
          (return (select `/Game/BP/Enum_AIFacingDirection` (`self.FacingDirection`) :`NewEnumerator0` "/Game/Sprites/BossDemon/BossDemonIdle/FB_BossDemonIdle.FB_BossDemonIdle" :`NewEnumerator1` "/Game/Sprites/BossDemon/BossDemonIdle/FB_BossDemonIdle.FB_BossDemonIdle" :!type "PaperFlipbook Object Reference")))))
    (:`NewEnumerator2`
      (return (select `bool` (<= (.x (- (`self.AvoidanceCoord`) (`self.K2_GetActorLocation`))) 0.0) :`false` "/Game/Sprites/BossDemon/BossDemonWalk/FB_BossDemonWalk.FB_BossDemonWalk" :`true` "/Game/Sprites/BossDemon/BossDemonWalk/FB_BossDemonWalk.FB_BossDemonWalk" :!type "PaperFlipbook Object Reference")))
    (:`NewEnumerator3`
      (if (or (== _returnvalue "/Game/Sprites/BossDemon/BossDemonAttackLeft/FB_BossDemonAttackLeft_Begin.FB_BossDemonAttackLeft_Begin") (== _returnvalue "/Game/Sprites/BossDemon/BossDemonAttackLeft/FB_BossDemonAttackLeft_Begin.FB_BossDemonAttackLeft_Begin"))
        (return (select `/Game/BP/Enum_AIFacingDirection` (`self.FacingDirection`) :`NewEnumerator0` "/Game/Sprites/BossDemon/BossDemonAttackLeft/FB_BossDemonAttackLeft_End.FB_BossDemonAttackLeft_End" :`NewEnumerator1` "/Game/Sprites/BossDemon/BossDemonAttackLeft/FB_BossDemonAttackLeft_End.FB_BossDemonAttackLeft_End" :!type "PaperFlipbook Object Reference"))
        (else
          (return (select `/Game/BP/Enum_AIFacingDirection` (`self.FacingDirection`) :`NewEnumerator0` "/Game/Sprites/BossDemon/BossDemonAttackLeft/FB_BossDemonAttackLeft_Begin.FB_BossDemonAttackLeft_Begin" :`NewEnumerator1` "/Game/Sprites/BossDemon/BossDemonAttackLeft/FB_BossDemonAttackLeft_Begin.FB_BossDemonAttackLeft_Begin" :!type "PaperFlipbook Object Reference")))))
    (:`NewEnumerator4`
      (return (select `byte` (`self.FacingDirection`) :`0` "/Game/Sprites/BossDemon/BossDemonIdle/FB_BossDemonIdle.FB_BossDemonIdle" :`1` "/Game/Sprites/BossDemon/BossDemonIdle/FB_BossDemonIdle.FB_BossDemonIdle" :!type "PaperFlipbook Object Reference")))))

(fn `GetChargeLocation`
  (returns (ChargeLocation :type "Vector Structure"))
  (locals (LeftImpactDistance :type "Float (double-precision)" :default 0.0) (LeftImpactLocation :type "Vector Structure" :default (0.0 0.0 0.0)) (RightImpactDistance :type "Float (double-precision)" :default 0.0) (RightImpactLocation :type "Vector Structure" :default (0.0 0.0 0.0)))
  (`|ExecutionSequence`
    (:`then_0`
      (bind _outhit (`KismetSystemLibrary.BoxTraceSingle` :`Start` (`self.K2_GetActorLocation`) :`End` (`KismetMathLibrary.MakeVector` (+ (.x (`self.K2_GetActorLocation`)) (* (.x (-1.0 0.0 0.0)) 500.0)) (.y (`self.K2_GetActorLocation`)) (.z (`self.K2_GetActorLocation`))) :`HalfSize` (`self.BoxExtent`) :`TraceChannel` "TraceTypeQuery1" :`bTraceComplex` true :`DrawDebugType` "ForDuration"))
      (bind (_bblockinghit _binitialoverlap _time _distance _location) (`GameplayStatics.BreakHitResult` _outhit))
      (if _bblockinghit
        (set `local.LeftImpactDistance` _distance)
        (set `local.LeftImpactLocation` _location)))
    (:`then_1`
      (bind _outhit_2 (`KismetSystemLibrary.BoxTraceSingle` :`Start` (`self.K2_GetActorLocation`) :`End` (`KismetMathLibrary.MakeVector` (+ (.x (`self.K2_GetActorLocation`)) (* (.x (1.0 0.0 0.0)) 500.0)) (.y (`self.K2_GetActorLocation`)) (.z (`self.K2_GetActorLocation`))) :`HalfSize` (`self.BoxExtent`) :`TraceChannel` "TraceTypeQuery1" :`bTraceComplex` true :`DrawDebugType` "ForDuration"))
      (bind (_bblockinghit_2 _binitialoverlap_2 _time_2 _distance_2 _location_2) (`GameplayStatics.BreakHitResult` _outhit_2))
      (if _bblockinghit_2
        (set `local.RightImpactDistance` _distance_2)
        (set `local.RightImpactLocation` _location_2)))
    (:`then_2`
      (`/Engine/EditorBlueprintResources/StandardMacros.CompareFloat` (`local.LeftImpactDistance`) (`local.RightImpactDistance`)
        (:`>`
          (return (`local.LeftImpactLocation`)))
        (:`==`
          (return (select `bool` (`KismetMathLibrary.RandomBool`) :`false` (`local.LeftImpactLocation`) :`true` (`local.RightImpactLocation`))))
        (:`<`
          (return (`local.RightImpactLocation`)))))))

(fn `UserConstructionScript`
  (`parent.UserConstructionScript`))

(fn `zAvoidance`
  (returns (Result :type Boolean))
  (locals (isCollidingRight :type Boolean) (isCollidingLeft :type Boolean) (IteratorDown :type Integer) (MaxIterations :type Integer) (IteratorUP :type Integer) (NewLocalVar_0 :type "Float (double-precision)" :default 48.0))
  (bind (_outhit _returnvalue) (`KismetSystemLibrary.BoxTraceSingle` :`Start` (`self.K2_GetActorLocation`) :`End` (`KismetMathLibrary.MakeVector` (+ (.x (`self.K2_GetActorLocation`)) (* (.x (`self.MovementDirection`)) (`local.NewLocalVar_0`))) 2.0 (.z (`self.K2_GetActorLocation`))) :`HalfSize` (8.0 0.0 8.0) :`TraceChannel` "TraceTypeQuery1" :`bTraceComplex` true :`DrawDebugType` "ForOneFrame"))
  (set `local.isCollidingRight` _returnvalue)
  (if (`local.isCollidingRight`)
    (while (and (`local.isCollidingRight`) (< (`local.IteratorUP`) (`local.MaxIterations`)))
      (`/Engine/EditorBlueprintResources/StandardMacros.IncrementInt` (`local.IteratorUP`)
        (:`  `
          (bind (_outhit_2 _returnvalue_2) (`KismetSystemLibrary.BoxTraceSingle` :`Start` (`KismetMathLibrary.MakeVector` (.x (`self.K2_GetActorLocation`)) 0.0 (+ (.z (`self.K2_GetActorLocation`)) (* (`KismetMathLibrary.Conv_IntToDouble` (`local.IteratorUP`)) 18.0))) :`End` (`KismetMathLibrary.MakeVector` (+ (.x (`self.K2_GetActorLocation`)) (* (.x (`self.MovementDirection`)) 48.0)) 2.0 (+ (.z (`self.K2_GetActorLocation`)) (* (`KismetMathLibrary.Conv_IntToDouble` (`local.IteratorUP`)) 18.0))) :`HalfSize` (8.0 0.0 8.0) :`TraceChannel` "TraceTypeQuery1" :`bTraceComplex` true :`DrawDebugType` "ForOneFrame"))
          (set `local.isCollidingRight` _returnvalue_2))))
    (while (and (`local.isCollidingRight`) (< (`local.IteratorDown`) (`local.MaxIterations`)))
      (`/Engine/EditorBlueprintResources/StandardMacros.IncrementInt` (`local.IteratorDown`)
        (:`  `
          (bind (_outhit_3 _returnvalue_3) (`KismetSystemLibrary.BoxTraceSingle` :`Start` (`KismetMathLibrary.MakeVector` (.x (`self.K2_GetActorLocation`)) 0.0 (+ (.z (`self.K2_GetActorLocation`)) (* (`KismetMathLibrary.Conv_IntToDouble` (`local.IteratorDown`)) -18.0))) :`End` (`KismetMathLibrary.MakeVector` (+ (.x (`self.K2_GetActorLocation`)) (* (.x (`self.MovementDirection`)) 48.0)) 2.0 (+ (.z (`self.K2_GetActorLocation`)) (* (`KismetMathLibrary.Conv_IntToDouble` (`local.IteratorDown`)) -18.0))) :`HalfSize` (8.0 0.0 8.0) :`TraceChannel` "TraceTypeQuery1" :`bTraceComplex` true :`DrawDebugType` "ForOneFrame"))
          (set `local.isCollidingRight` _returnvalue_3))))
    (`|ExecutionSequence`
      (:`then_0`
        (`/Engine/EditorBlueprintResources/StandardMacros.CompareInt` (`local.IteratorUP`) (`local.IteratorDown`)
          (:`>`
            (set `self.AvoidanceCoord` (`KismetMathLibrary.MakeVector` (.x (`self.K2_GetActorLocation`)) 2.0 (+ (.z (`self.K2_GetActorLocation`)) (* (`KismetMathLibrary.Conv_IntToDouble` (`local.IteratorDown`)) -18.0)))))
          (:`==`
            (set `self.AvoidanceCoord` (`KismetMathLibrary.MakeVector` (.x (`self.K2_GetActorLocation`)) 2.0 (+ (.z (`self.K2_GetActorLocation`)) (* (`KismetMathLibrary.Conv_IntToDouble` (`local.IteratorUP`)) 18.0 (`KismetMathLibrary.Conv_IntToDouble` (select `bool` (`KismetMathLibrary.RandomBool`) :`false` -1 :`true` 1)))))))
          (:`<`
            (set `self.AvoidanceCoord` (`KismetMathLibrary.MakeVector` (.x (`self.K2_GetActorLocation`)) 2.0 (+ (.z (`self.K2_GetActorLocation`)) (* (`KismetMathLibrary.Conv_IntToDouble` (`local.IteratorUP`)) 18.0)))))))
      (:`then_1`
        (`KismetSystemLibrary.DrawDebugBox` (`self.AvoidanceCoord`) (8.0 0.0 8.0) (struct :`R` 0.177915 :`G` 1.0 :`B` 0.005004 :`A` 1.0) (struct) 5.0 2.0)
        (set `self.State` "NewEnumerator2")
        (return true)))
    (else
      (return false))))