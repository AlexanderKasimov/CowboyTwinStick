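; Test squad manager that hands out formation grid spots to the melee cultists in the level.
; BeginPlay builds a four-spot attack line and a four-spot second column, split by X/Z side, and collects all cultists.
; Each Tick gives spotless cultists the first free spot, attack line first, and moves cultists off the attack column into free attack spots.
; FreeGridSpot marks spots free again, and ReportDeath removes cultists from the squad.
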(event `/Game/BP/AICommunicationInterface.ReportDeath`
  (params (DeadActor :type "Actor Object Reference"))
  (`KismetArrayLibrary.Array_RemoveItem` (`self.CultistArray`) (cast `/Game/BP/Testing/BP_NewAITest_MeleeCultist` DeadActor :!pure true)))

(event `/Game/BP/AICommunicationInterface.FreeGridSpot`
  (params (GridSpot :type "/Game/BP/Testing/Struct_GridSpot Structure"))
  (bind _returnvalue (`KismetArrayLibrary.Array_Find` (`self.GridSpotArray`) GridSpot))
  (bind _returnvalue_2 (`KismetArrayLibrary.Array_Find` (`self.AttackLineGridSpotArray`) GridSpot))
  ;[1 1 1] Refactor ASAP
  (set `self.NewVar_0` _returnvalue_2)
  (if (not (== _returnvalue_2 -1))
    (bind _structout (setmembers `/Game/BP/Testing/Struct_GridSpot` :`StructRef` GridSpot :`isFree` true))
    (`KismetArrayLibrary.Array_Set` (`self.AttackLineGridSpotArray`) (`self.NewVar_0`) _structout)
    (`KismetSystemLibrary.PrintString` "Hello")
    (elif (not (== _returnvalue -1))
      (bind _structout_2 (setmembers `/Game/BP/Testing/Struct_GridSpot` :`StructRef` GridSpot :`isFree` true))
      (`KismetArrayLibrary.Array_Set` (`self.GridSpotArray`) _returnvalue _structout_2)
      (`KismetSystemLibrary.PrintString` "Free!")
      (else
        (`KismetSystemLibrary.PrintString` "Error!")))))

(event `self.ReceiveBeginPlay`
  (`self.GenerateGrid`)
  (bind _outactors (`GameplayStatics.GetAllActorsOfClass` "/Game/BP/Testing/BP_NewAITest_MeleeCultist.BP_NewAITest_MeleeCultist_C"))
  (set `self.CultistArray` _outactors))

(event `self.ReceiveTick`
  (params (DeltaSeconds :type "Float (single-precision)"))
  (bind (_return _gridspot _index) (`self.GetFreeGridSpot` (`self.GridSpotArray`)))
  (bind (_return_2 _gridspot_2 _index_2) (`self.GetFreeGridSpot` (`self.AttackLineGridSpotArray`)))
  (bind (_return_3 _gridspot_3 _index_3) (`self.GetFreeGridSpot` (`self.AttackLineGridSpotArray`)))
  (for _array_element (`self.CultistArray`)
    (if (`/Game/BP/Testing/BP_NewAITest_MeleeCultist.hasGridSpot` _array_element)
      (if _return_2
        (if (not (`/Game/BP/Testing/BP_NewAITest_MeleeCultist.onAttackColumn` _array_element))
          (bind _structout (setmembers `/Game/BP/Testing/Struct_GridSpot` :`StructRef` _gridspot_2 :`isFree` false))
          (`KismetArrayLibrary.Array_Set` (`self.AttackLineGridSpotArray`) _index_2 _structout)
          (message `/Game/BP/AICommunicationInterface.SetGridSpot` _array_element _structout)))
      (elif _return_3
        (bind _structout_2 (setmembers `/Game/BP/Testing/Struct_GridSpot` :`StructRef` _gridspot_3 :`isFree` false))
        (`KismetArrayLibrary.Array_Set` (`self.AttackLineGridSpotArray`) _index_3 _structout_2)
        (message `/Game/BP/AICommunicationInterface.SetGridSpot` _array_element _structout_2)
        (elif _return
          (bind _structout_3 (setmembers `/Game/BP/Testing/Struct_GridSpot` :`StructRef` _gridspot :`isFree` false))
          (`KismetArrayLibrary.Array_Set` (`self.GridSpotArray`) _index _structout_3)
          (message `/Game/BP/AICommunicationInterface.SetGridSpot` _array_element _structout_3))))))

(fn `GenerateGrid`
  (`|ExecutionSequence`
    (:`then_0`
      (`KismetArrayLibrary.Array_Add` (`self.AttackLineGridSpotArray`) (make `/Game/BP/Testing/Struct_GridSpot` "NewEnumerator1"))
      (`KismetArrayLibrary.Array_Add` (`self.AttackLineGridSpotArray`) (make `/Game/BP/Testing/Struct_GridSpot` "NewEnumerator1" "NewEnumerator1")))
    (:`then_1`
      (`KismetArrayLibrary.Array_Add` (`self.AttackLineGridSpotArray`) (make `/Game/BP/Testing/Struct_GridSpot` "NewEnumerator0"))
      (`KismetArrayLibrary.Array_Add` (`self.AttackLineGridSpotArray`) (make `/Game/BP/Testing/Struct_GridSpot` "NewEnumerator0" "NewEnumerator1")))
    (:`then_2`
      (`KismetArrayLibrary.Array_Add` (`self.GridSpotArray`) (make `/Game/BP/Testing/Struct_GridSpot` "NewEnumerator1" "NewEnumerator0" 2))
      (`KismetArrayLibrary.Array_Add` (`self.GridSpotArray`) (make `/Game/BP/Testing/Struct_GridSpot` "NewEnumerator1" "NewEnumerator1" 2)))
    (:`then_3`
      (`KismetArrayLibrary.Array_Add` (`self.GridSpotArray`) (make `/Game/BP/Testing/Struct_GridSpot` "NewEnumerator0" "NewEnumerator0" 2))
      (`KismetArrayLibrary.Array_Add` (`self.GridSpotArray`) (make `/Game/BP/Testing/Struct_GridSpot` "NewEnumerator0" "NewEnumerator1" 2)))))

(fn `GetFreeGridSpot`
  (params (Pool :type "Array of /Game/BP/Testing/Struct_GridSpot Structure"))
  (returns (Return :type Boolean) (GridSpot :type "/Game/BP/Testing/Struct_GridSpot Structure") (Index :type Integer))
  (for (_array_element _array_index) Pool
    (if (`.isFree_15_6CBAA09A48F22CCA698904BF7A3EEA08` (break `/Game/BP/Testing/Struct_GridSpot` _array_element))
      (return true _array_element _array_index)))
  (return false (struct) -1))

(fn `UserConstructionScript`)