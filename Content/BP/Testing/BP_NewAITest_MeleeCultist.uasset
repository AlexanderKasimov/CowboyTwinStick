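; Test melee cultist AI that moves directly toward a point offset along X from the player pawn.
; Each Tick it caches player pawn 0 and sets a facing enum from which X side the player is on.
; It then steps toward the offset point with a swept SetActorLocation, without pathfinding, and draws debug visuals for target and movement.
; The offset ignores facing; a sign-based offset calculation is left unconnected.
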(event `self.ReceiveTick`
  (params (DeltaSeconds :type "Float (single-precision)"))
  (bind _returnvalue (`GameplayStatics.GetPlayerPawn` 0))
  (`|ExecutionSequence`
    (:`then_0`
      (`/Engine/EditorBlueprintResources/StandardMacros.IsValid` _returnvalue
        (:`Is Valid`
          (set `self.PlayerPawn` (`GameplayStatics.GetPlayerPawn` 0))
          (if (<= (.x (- (`self.K2_GetActorLocation` _returnvalue) (`self.K2_GetActorLocation`))) 0.0)
            (set `self.FacingDirection` "NewEnumerator0")
            (else
              (set `self.FacingDirection` "NewEnumerator1"))))))
    (:`then_1`
      (bind _output_get (set `self.PlayerPositionWithOffset` (- (`self.K2_GetActorLocation` (`self.PlayerPawn`)) (`KismetMathLibrary.MakeVector` (`self.PlayerPositionOffset`)))))
      (`/Game/BP/DebugFunctionLibrary.DebugBox` true _output_get)
      (set `self.MovementDirection` (`KismetMathLibrary.Normal` (- (`self.PlayerPositionWithOffset`) (`self.K2_GetActorLocation`))))
      (`KismetSystemLibrary.DrawDebugArrow` (`self.K2_GetActorLocation`) (+ (`self.K2_GetActorLocation`) (* (`self.MovementDirection`) (`self.MovementSpeed`))) 5.0 (struct :`R` 1.0 :`B` 0.035352 :`A` 1.0) 0.0 1.0)
      (`self.K2_SetActorLocation` (+ (`self.K2_GetActorLocation`) (* (`self.MovementDirection`) (* (`GameplayStatics.GetWorldDeltaSeconds`) (`self.MovementSpeed`)))) true))))

(fn `UserConstructionScript`)