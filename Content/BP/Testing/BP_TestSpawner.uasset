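; Test spawner that adds melee cultists while activated, keeping their count up to a maximum.
; Activate starts a looping timer that calls Spawn at the spawn rate, and Deactivate clears it.
; Spawn reads the squad manager's cultist array and infers each side's population from facing direction.
; It spawns a pair, or one if only one slot remains, at the less crowded side's points, choosing randomly on ties.
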(event `Activate`
  (bind _returnvalue (`KismetSystemLibrary.K2_SetTimer` null "Spawn" (`self.SpawnRate`) true))
  (set `self.SpawnTimerHandle` _returnvalue))

(event `Deactivate`
  (`KismetSystemLibrary.K2_ClearAndInvalidateTimerHandle` (`self.SpawnTimerHandle`)))

(fn `Spawn`
  (locals (CulstistArray :type "Array of /Game/BP/Testing/BP_NewAITest_MeleeCultist Object Reference") (RightSideCharCount :type Integer) (LeftSideCharCount :type Integer) (CurCharCount :type Integer :default 0) (SpotSide :type "/Game/BP/Enum_AIFacingDirection Enum") (CurSpawnPoints :type "Array of TargetPoint Object Reference"))
  (bind _outactors (`GameplayStatics.GetAllActorsOfClass` "/Game/BP/Testing/BP_NewAITest_SquadManager.BP_NewAITest_SquadManager_C"))
  (bind _output_get (set `local.CulstistArray` (`/Game/BP/Testing/BP_NewAITest_SquadManager.CultistArray` (`|GetArrayItem` _outactors))))
  (bind _output_get_2 (set `local.CurCharCount` (`KismetArrayLibrary.Array_Length` _output_get)))
  (if (< _output_get_2 (`self.MaxCharacters`))
    (for _array_element (`local.CulstistArray`)
      (switch `/Game/BP/Enum_AIFacingDirection` (`/Game/BP/Testing/BP_NewAITest_MeleeCultist.FacingDirection` _array_element)
        (:`NewEnumerator0`
          (`/Engine/EditorBlueprintResources/StandardMacros.IncrementInt` (`local.RightSideCharCount`)))
        (:`NewEnumerator1`
          (`/Engine/EditorBlueprintResources/StandardMacros.IncrementInt` (`local.LeftSideCharCount`)))))
    (`|ExecutionSequence`
      (:`then_0`
        (`/Engine/EditorBlueprintResources/StandardMacros.CompareInt` (`local.RightSideCharCount`) (`local.LeftSideCharCount`)
          (:`>`
            (set `local.CurSpawnPoints` (`self.LeftSpawnPoints`)))
          (:`==`
            (set `local.CurSpawnPoints` (select `bool` (`KismetMathLibrary.RandomBool`) :`false` (`self.LeftSpawnPoints`) :`true` (`self.RightSpawnPoints`))))
          (:`<`
            (set `local.CurSpawnPoints` (`self.RightSpawnPoints`)))))
      (:`then_1`
        (if (<= (+ (`local.CurCharCount`) 2) (`self.MaxCharacters`))
          (for _index (range 2)
            (bind _returnvalue (`|SpawnActorFromClass` "/Game/BP/Testing/BP_NewAITest_MeleeCultist.BP_NewAITest_MeleeCultist_C" (`KismetMathLibrary.Conv_VectorToTransform` (`self.K2_GetActorLocation` (`|GetArrayItem` (`local.CurSpawnPoints`) _index))) "AlwaysSpawn" "OverrideRootScale" null null)))
          (else
            (for _index_2 (range 1)
              (bind _returnvalue_2 (`|SpawnActorFromClass` "/Game/BP/Testing/BP_NewAITest_MeleeCultist.BP_NewAITest_MeleeCultist_C" (`KismetMathLibrary.Conv_VectorToTransform` (`self.K2_GetActorLocation` (`|GetArrayItem` (`local.CurSpawnPoints`) _index_2))) "AlwaysSpawn" "OverrideRootScale" null null)))))))))

(fn `UserConstructionScript`)