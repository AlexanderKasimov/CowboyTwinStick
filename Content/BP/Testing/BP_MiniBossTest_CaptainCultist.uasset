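; Test mini-boss Captain Cultist: a flipbook enemy that, once activated, becomes vulnerable and chases the player on the X/Z plane.
; Tick drives facing and movement, with cooldown-gated speed-boost charges, switching to attack when close.
; Flipbook completion chains attack phases, firing a box-trace sword hit between them, and on death notifies the game mode and destroys the actor.
; Blocking recharges on a timer; squad grid-spot logic is left unused.
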(event `Activate`
  (set `self.CanMove` true)
  (set `/Game/BP/BP_BaseHealthComponent.isImmortal` false (`self.BP_BaseHealthComponent`)))

(event `self.ReceiveBeginPlay`)

(event `/Game/BP/IDamagable.HandleDeath`
  (params (DeathCause :type "/Game/BP/Enum_DeathCause Enum" :default "NewEnumerator0"))
  (set `self.DeathCause` DeathCause)
  (set `self.State` "NewEnumerator4")
  (bind _flipbook (`self.GetAnimation`))
  (`PaperFlipbookComponent.SetFlipbook` (`self.PaperFlipbook`) _flipbook)
  (`PaperFlipbookComponent.SetLooping` (`self.PaperFlipbook`) false)
  (`PaperFlipbookComponent.PlayFromStart` (`self.PaperFlipbook`)))

(event `/Game/BP/AICommunicationInterface.SetGridSpot`
  (params (GridSpot :type "/Game/BP/Testing/Struct_GridSpot Structure")))

(event `/Game/BP/AICommunicationInterface.DebugGrid`
  (params (SpotGrid :type "Array of /Game/BP/Testing/Struct_GridSpot Structure (by ref)")))

(event `self.ReceiveTick`
  (params (DeltaSeconds :type "Float (single-precision)"))
  (bind _returnvalue (`GameplayStatics.GetPlayerPawn` 0))
  (`|ExecutionSequence`
    (:`then_0`
      (`/Engine/EditorBlueprintResources/StandardMacros.IsValid` _returnvalue
        (:`Is Valid`
          ;[1 1 1] Может быть null
          (set `self.PlayerPawn` (`GameplayStatics.GetPlayerPawn` 0))
          (if (<= (.x (- (`self.K2_GetActorLocation` _returnvalue) (`self.K2_GetActorLocation`))) 0.0)
            (set `self.FacingDirection` "NewEnumerator0")
            (else
              (set `self.FacingDirection` "NewEnumerator1"))))))
    (:`then_1`
      (`/Engine/EditorBlueprintResources/StandardMacros.IsValid` (`GameplayStatics.GetPlayerPawn` 0)
        (:`Is Valid`
          (switch `/Game/BP/Enum_AiStates` (`self.State`)
            (:`NewEnumerator1`
              (if (`self.CanMove`)
                (bind _output_get (set `self.GridSpotLocation` (`self.K2_GetActorLocation` (`self.PlayerPawn`))))
                (`/Game/BP/DebugFunctionLibrary.DebugBox` (`self.DebugMode`) _output_get)
                (if (or (> (`KismetMathLibrary.Abs` (.x (- (`self.K2_GetActorLocation`) (`self.K2_GetActorLocation` (`self.PlayerPawn`))))) 25.0) false (> (`KismetMathLibrary.Abs` (.z (- (`self.K2_GetActorLocation`) (`self.K2_GetActorLocation` (`self.PlayerPawn`))))) 20.0))
                  (if (not (and (> (`KismetMathLibrary.VSize` (- (`self.K2_GetActorLocation`) (`self.K2_GetActorLocation` (`self.PlayerPawn`)))) 40.0) (`self.canCharge`)))
                    (set `self.MovementDirection` (`KismetMathLibrary.Normal` (- (`self.GridSpotLocation`) (`self.K2_GetActorLocation`))))
                    (`/Game/BP/DebugFunctionLibrary.DebugArrow` (`self.DebugMode`) (`self.K2_GetActorLocation`) (+ (`self.K2_GetActorLocation`) (* (`self.MovementDirection`) (`self.MovementSpeed`))))
                    (`self.K2_SetActorLocation` (+ (`self.K2_GetActorLocation`) (* (`self.MovementDirection`) (* (`GameplayStatics.GetWorldDeltaSeconds`) (`self.MovementSpeed`)))) true)
                    (else
                      (set `self.canCharge` false)
                      (set `self.MovementSpeed` (`self.MovementSpeedCharge`))
                      (`KismetSystemLibrary.K2_SetTimerDelegate` (delegate `EndCharge`) (`self.ChargeDuration`))
                      (`KismetSystemLibrary.K2_SetTimerDelegate` (delegate `ResetCharge`) (`self.ChargeCooldown`))))
                  (else
                    (set `self.State` "NewEnumerator3")
                    (bind _flipbook (`self.GetAnimation`))
                    (`PaperFlipbookComponent.SetFlipbook` (`self.PaperFlipbook`) _flipbook)
                    (`PaperFlipbookComponent.SetLooping` (`self.PaperFlipbook`) false)
                    (`PaperFlipbookComponent.PlayFromStart` (`self.PaperFlipbook`))))))))))
    (:`then_2`
      (switch `/Game/BP/Enum_AiStates` (`self.State`)
        (:`NewEnumerator1`
          _)
        (:`NewEnumerator2`
          _))
      (bind _flipbook_2 (`self.GetAnimation`))
      (`PaperFlipbookComponent.SetFlipbook` (`self.PaperFlipbook`) _flipbook_2)
      (`PaperFlipbookComponent.SetLooping` (`self.PaperFlipbook`) true))))

(event `EndCharge`
  (set `self.MovementSpeed` (`self.MovementSpeedNormal`)))

(event `ResetCharge`
  (set `self.canCharge` true)
  (`KismetSystemLibrary.PrintString` "ResetedCharge"))

(event `self.PaperFlipbook.OnFinishedPlaying`
  (switch `/Game/BP/Enum_AiStates` (`self.State`)
    (:`NewEnumerator3`
      (if (or (== (`PaperFlipbookComponent.GetFlipbook` (`self.PaperFlipbook`)) "/Game/Sprites/Cultist/CultistAttackLeft/FB_CultistAttack_Begin.FB_CultistAttack_Begin") (== (`PaperFlipbookComponent.GetFlipbook` (`self.PaperFlipbook`)) "/Game/Sprites/Cultist/CultistAttackRight/FB_CultistAttackRight_Begin.FB_CultistAttackRight_Begin"))
        (`|ExecutionSequence`
          (:`then_0`
            (bind _flipbook (`self.GetAnimation`))
            (`PaperFlipbookComponent.SetFlipbook` (`self.PaperFlipbook`) _flipbook)
            (`PaperFlipbookComponent.PlayFromStart` (`self.PaperFlipbook`)))
          (:`then_1`
            (`self.Attack`)))
        (elif (or (== (`PaperFlipbookComponent.GetFlipbook` (`self.PaperFlipbook`)) "/Game/Sprites/Cultist/CultistAttackLeft/FB_CultistAttack_End.FB_CultistAttack_End") (== (`PaperFlipbookComponent.GetFlipbook` (`self.PaperFlipbook`)) "/Game/Sprites/Cultist/CultistAttackRight/FB_CultistAttackRight_End.FB_CultistAttackRight_End"))
          (set `self.State` "NewEnumerator1")
          (`PaperFlipbookComponent.PlayFromStart` (`self.PaperFlipbook`)))))
    (:`NewEnumerator4`
      (`/Game/BP/GM_BaseTwinStick.Boss Died` (cast `/Game/BP/GM_BaseTwinStick` (`GameplayStatics.GetGameMode`) :!pure true))
      (`self.K2_DestroyActor`))))

(event `/Game/BP/IDamagable.HandleBlock`
  (set `/Game/BP/BP_BaseHealthComponent.canBlock` false (`self.BP_BaseHealthComponent`))
  (`KismetSystemLibrary.K2_SetTimerDelegate` (delegate `ResetBlock`) (`self.BlockCooldown`)))

(event `ResetBlock`
  (set `/Game/BP/BP_BaseHealthComponent.canBlock` true (`self.BP_BaseHealthComponent`))
  (`KismetSystemLibrary.PrintString` "Reseted"))

(fn `Attack`
  (bind _returnvalue (+ (`self.K2_GetActorLocation`) (* (`KismetMathLibrary.Normal` (`KismetMathLibrary.MakeVector` (.x (- (`self.K2_GetActorLocation` (`GameplayStatics.GetPlayerPawn` 0)) (`self.K2_GetActorLocation`))))) 20.0)))
  (`/Engine/EditorBlueprintResources/StandardMacros.IsValid` (`GameplayStatics.GetPlayerPawn` 0)
    (:`Is Valid`
      (bind _outhit (`KismetSystemLibrary.BoxTraceSingle` :`Start` _returnvalue :`End` _returnvalue :`HalfSize` (`KismetMathLibrary.MakeVector` (`self.AttackLength`) 0.0 (`self.AttackWidth`)) :`TraceChannel` "TraceTypeQuery1" :`bTraceComplex` true :`DrawDebugType` (select `bool` false :`true` "ForDuration" :!type "EDrawDebugTrace Enum")))
      (bind (_bblockinghit _binitialoverlap _time _distance _location _impactpoint _normal _impactnormal _physmat _hitactor) (`GameplayStatics.BreakHitResult` _outhit))
      (if _bblockinghit
        (bind _returnvalue_2 (`self.GetComponentByClass` _hitactor "/Game/BP/BP_BaseHealthComponent.BP_BaseHealthComponent_C"))
        (`/Engine/EditorBlueprintResources/StandardMacros.IsValid` _returnvalue_2
          (:`Is Valid`
            (message `/Game/BP/IDamagable.HandleDamage` _returnvalue_2 (`self.AttackDamage`) "NewEnumerator1")))))))

(fn `CalculateGridSpotLocation`
  (returns (Location :type "Vector Structure"))
  (locals (SignX :type "Float (double-precision)") (SignZ :type "Float (double-precision)") (OffsetX :type "Float (double-precision)" :default 30.0) (OffsetZ :type "Float (double-precision)" :default 40.0))
  (bind (_sidex _sidez _column _row) (break `/Game/BP/Testing/Struct_GridSpot` (`self.GridSpot`)))
  (set `local.SignX` (select `/Game/BP/Enum_AIFacingDirection` _sidex :`NewEnumerator0` -1.0 :`NewEnumerator1` 1.0 :!type "Float (single-precision)"))
  (set `local.SignZ` (select `/Game/BP/Testing/Enum_SpotSideZ` _sidez :`NewEnumerator0` 1.0 :`NewEnumerator1` -1.0 :!type "Float (single-precision)"))
  (`/Engine/EditorBlueprintResources/StandardMacros.IsValid` (`GameplayStatics.GetPlayerPawn` 0)
    (:`Is Valid`
      (return (+ (`self.K2_GetActorLocation` (`GameplayStatics.GetPlayerPawn` 0)) (`KismetMathLibrary.MakeVector` (* (`local.OffsetX`) (`KismetMathLibrary.Conv_IntToDouble` _column) (`local.SignX`)) 0.0 (+ (* (/ (`local.OffsetZ`) 2.0) (`local.SignZ`)) (* (`local.OffsetZ`) (`KismetMathLibrary.Conv_IntToDouble` (- _row 1)) (`local.SignZ`)))))))))

(fn `DebugGridTest`
  (params (Array :type "Array of /Game/BP/Testing/Struct_GridSpot Structure"))
  (locals (SignX :type "Float (double-precision)" :default 0.0) (SignZ :type "Float (double-precision)" :default 0.0) (OffsetX :type "Float (double-precision)" :default 20.0) (OffsetZ :type "Float (double-precision)" :default 20.0))
  (for _array_element Array
    (bind (_sidex _sidez _column _row) (break `/Game/BP/Testing/Struct_GridSpot` _array_element))
    (set `local.SignX` (select `/Game/BP/Enum_AIFacingDirection` _sidex :`NewEnumerator0` -1.0 :`NewEnumerator1` 1.0 :!type "Float (single-precision)"))
    (set `local.SignZ` (select `/Game/BP/Testing/Enum_SpotSideZ` _sidez :`NewEnumerator0` 1.0 :`NewEnumerator1` -1.0 :!type "Float (single-precision)"))
    (`/Engine/EditorBlueprintResources/StandardMacros.IsValid` (`GameplayStatics.GetPlayerPawn` 0)
      (:`Is Valid`
        (`/Game/BP/DebugFunctionLibrary.DebugBox` true (+ (`self.K2_GetActorLocation` (`GameplayStatics.GetPlayerPawn` 0)) (`KismetMathLibrary.MakeVector` (* (`local.OffsetX`) (`KismetMathLibrary.Conv_IntToDouble` _column) (`local.SignX`)) 0.0 (+ (* (/ (`local.OffsetZ`) 2.0) (`local.SignZ`)) (* (`local.OffsetZ`) (`KismetMathLibrary.Conv_IntToDouble` (- _row 1)) (`local.SignZ`))))) (2.0 0.0 2.0) (struct :`R` 0.176471 :`G` 1.0 :`B` 0.003922 :`A` 1.0) 5.0)))))

(fn `GetAnimation`
  (returns (Flipbook :type "PaperFlipbook Object Reference"))
  (bind _returnvalue (`PaperFlipbookComponent.GetFlipbook` (`self.PaperFlipbook`)))
  (switch `/Game/BP/Enum_AiStates` (`self.State`)
    (:`NewEnumerator1`
      _)
    (:`NewEnumerator2`
      _)
    (:`NewEnumerator3`
      (if (or (== _returnvalue "/Game/Sprites/Cultist/CultistAttackLeft/FB_CultistAttack_Begin.FB_CultistAttack_Begin") (== _returnvalue "/Game/Sprites/Cultist/CultistAttackRight/FB_CultistAttackRight_Begin.FB_CultistAttackRight_Begin"))
        (return (select `/Game/BP/Enum_AIFacingDirection` (`self.FacingDirection`) :`NewEnumerator0` "/Game/Sprites/Cultist/CultistAttackLeft/FB_CultistAttack_End.FB_CultistAttack_End" :`NewEnumerator1` "/Game/Sprites/Cultist/CultistAttackRight/FB_CultistAttackRight_End.FB_CultistAttackRight_End" :!type "PaperFlipbook Object Reference"))
        (else
          (return (select `/Game/BP/Enum_AIFacingDirection` (`self.FacingDirection`) :`NewEnumerator0` "/Game/Sprites/Cultist/CultistAttackLeft/FB_CultistAttack_Begin.FB_CultistAttack_Begin" :`NewEnumerator1` "/Game/Sprites/Cultist/CultistAttackRight/FB_CultistAttackRight_Begin.FB_CultistAttackRight_Begin" :!type "PaperFlipbook Object Reference")))))
    (:`NewEnumerator4`
      (switch `/Game/BP/Enum_DeathCause` (`self.DeathCause`)
        (:`NewEnumerator0`
          _)
        (:`NewEnumerator1`
          _)
        (:`NewEnumerator2`
          (return (select `/Game/BP/Enum_AIFacingDirection` (`self.FacingDirection`) :`NewEnumerator0` "/Game/Sprites/Cultist/CultistDeaths/CultistDeath_03/FB_CultistDeath_03.FB_CultistDeath_03" :`NewEnumerator1` "/Game/Sprites/Cultist/CultistDeaths/CultistDeath_03_Right/FB_CultistDeath_03_Right.FB_CultistDeath_03_Right" :!type "PaperFlipbook Object Reference"))))
      (if (`KismetMathLibrary.RandomBool`)
        (return (select `/Game/BP/Enum_AIFacingDirection` (`self.FacingDirection`) :`NewEnumerator0` "/Game/Sprites/Cultist/CultistDeaths/CultistDeath_01/FB_CultistDeath_01.FB_CultistDeath_01" :`NewEnumerator1` "/Game/Sprites/Cultist/CultistDeaths/CultistDeath_01_Right/FB_CultistDeath_01_Right.FB_CultistDeath_01_Right" :!type "PaperFlipbook Object Reference"))
        (else
          (return (select `/Game/BP/Enum_AIFacingDirection` (`self.FacingDirection`) :`NewEnumerator0` "/Game/Sprites/Cultist/CultistDeaths/CultistDeath_02/FB_CultistDeath_02.FB_CultistDeath_02" :`NewEnumerator1` "/Game/Sprites/Cultist/CultistDeaths/CultistDeath_02_Right/FB_CultistDeath_02_Right.FB_CultistDeath_02_Right" :!type "PaperFlipbook Object Reference"))))))
  (if true
    (return (select `/Game/BP/Enum_AIFacingDirection` (`self.FacingDirection`) :`NewEnumerator0` "/Game/Sprites/Cultist/CultistWalkLeft/FB_CultistWalk.FB_CultistWalk" :`NewEnumerator1` "/Game/Sprites/Cultist/CultistWalkRight/FB_CultistWalkRight.FB_CultistWalkRight" :!type "PaperFlipbook Object Reference"))))

(fn `UserConstructionScript`)