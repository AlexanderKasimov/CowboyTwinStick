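; BP_BaseProjectile is a base projectile actor with a Paper2D sprite that travels in a straight line.
; Each Tick moves it by Direction times Speed with a swept SetActorLocation, without delta-time scaling, so velocity depends on frame rate.
; The construction script pitches the sprite 90 degrees and shrinks it to quarter scale.
; The file contains no hit, damage or lifetime logic.
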(event `self.ReceiveTick`
  (params (DeltaSeconds :type "Float (single-precision)"))
  (`self.K2_SetActorLocation` (+ (`self.K2_GetActorLocation`) (* (`self.Direction`) (`self.Speed`))) true))

(fn `UserConstructionScript`
  (`SceneComponent.K2_SetRelativeRotation` (`self.PaperSprite`) (struct :`Roll` 90.0) false false)
  (`SceneComponent.SetWorldScale3D` (`self.PaperSprite`) (0.25 0.25 0.25)))