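; Base player controller that manages game modes, UI screens and level transitions.
; Mode functions create or remove menu, dialog and end/lose widgets, toggle pawn and UI/game input, and set GameState.
; PlayCutsceneF shows a frame-based widget advanced by Use, while dialog paragraph-advance logic is disconnected.
; Init stores level names and a streaming flag; restart reloads the sublevel or reopens the level, and LoadMainMenu streams in the menu.
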(event `self.ReceiveTick`
  (params (DeltaSeconds :type "Float (single-precision)")))

(event `InputAction|Use`
  (params (Key :type "Key Structure"))
  (:`Pressed`
    (`/Engine/EditorBlueprintResources/StandardMacros.IsValid` (`self.CutsceneWidget`)
      (:`Is Valid`
        (`/Game/BP/Testing/Cutscene.NextFrame` (`self.CutsceneWidget`))))))

(event `/Game/BP/Testing/Cutscene.EndCutscene`
  (`self.EndCutscene(F)`))

(event `Restart Level`
  (if (`self.isStreamingEnabled`)
    (`self.LevelRestarting`)
    (`GameplayStatics.UnloadStreamLevel` (`self.CurLevel`))
    (`GameplayStatics.LoadStreamLevel` (`self.CurLevel`) true true)
    (else
      (`GameplayStatics.OpenLevel` (`self.CurLevel`)))))

(event `LoadMainMenu`
  (`GameplayStatics.UnloadStreamLevel` (`self.CurLevel`))
  (`GameplayStatics.LoadStreamLevel` "MainMenu" true true))

(fn `BattleMode`
  (bind _returnvalue (`GameplayStatics.GetPlayerPawn` 0))
  (`|ExecutionSequence`
    (:`then_0`
      (`/Engine/EditorBlueprintResources/StandardMacros.IsValid` (`self.DialogWidgetRef`)
        (:`Is Valid`
          (`Widget.RemoveFromParent` (`self.DialogWidgetRef`)))))
    (:`then_1`
      (`/Engine/EditorBlueprintResources/StandardMacros.IsValid` (`self.MainMenuWidgetRef`)
        (:`Is Valid`
          (`Widget.RemoveFromParent` (`self.MainMenuWidgetRef`)))))
    (:`then_2`
      (`/Engine/EditorBlueprintResources/StandardMacros.IsValid` _returnvalue
        (:`Is Valid`
          (`self.EnableInput` _returnvalue self)
          (`WidgetBlueprintLibrary.SetInputMode_GameOnly` self)
          (set `self.GameState` "NewEnumerator3"))))))

(fn `CutsceneMode`
  (params (DialogTextName :type "/Game/BP/Enum_TextArrayNames Enum" :default "NewEnumerator0"))
  (locals (LocalDialogTextName :type "/Game/BP/Enum_TextArrayNames Enum" :default "NewEnumerator0"))
  (bind _returnvalue (`GameplayStatics.GetPlayerPawn` 0))
  (set `local.LocalDialogTextName` DialogTextName)
  (`/Engine/EditorBlueprintResources/StandardMacros.IsValid` (`self.MainMenuWidgetRef`)
    (:`Is Valid`
      (`Widget.RemoveFromParent` (`self.MainMenuWidgetRef`))
      (`/Engine/EditorBlueprintResources/StandardMacros.IsValid` _returnvalue
        (:`Is Valid`
          (`self.DisableInput` _returnvalue null)
          (bind _returnvalue_2 (`|CreateWidget` "/Game/UI/DialogWidget.DialogWidget_C" null (`local.LocalDialogTextName`)))
          (bind _output_get (set `self.DialogWidgetRef` _returnvalue_2))
          (`UserWidget.AddToViewport` _output_get 0)
          (`WidgetBlueprintLibrary.SetInputMode_GameOnly` self)
          (set `self.GameState` "NewEnumerator1"))))))

(fn `DialogMode`
  (params (DialogTextName :type "/Game/BP/Enum_TextArrayNames Enum" :default "NewEnumerator0"))
  (locals (LocalDialogTextName :type "/Game/BP/Enum_TextArrayNames Enum"))
  (bind _returnvalue (`GameplayStatics.GetPlayerPawn` 0))
  (set `local.LocalDialogTextName` DialogTextName)
  (`/Engine/EditorBlueprintResources/StandardMacros.IsValid` (`self.MainMenuWidgetRef`)
    (:`Is Valid`
      (`Widget.RemoveFromParent` (`self.MainMenuWidgetRef`))
      (`/Engine/EditorBlueprintResources/StandardMacros.IsValid` _returnvalue
        (:`Is Valid`
          (`self.DisableInput` _returnvalue null)
          (bind _returnvalue_2 (`|CreateWidget` "/Game/UI/DialogWidget.DialogWidget_C" null (`local.LocalDialogTextName`)))
          (bind _output_get (set `self.DialogWidgetRef` _returnvalue_2))
          (`UserWidget.AddToViewport` _output_get 0)
          (`WidgetBlueprintLibrary.SetInputMode_GameOnly` self)
          (set `self.GameState` "NewEnumerator4"))))))

(fn `EndCutscene(F)`
  (bind _returnvalue (`GameplayStatics.GetPlayerPawn` 0))
  (`/Engine/EditorBlueprintResources/StandardMacros.IsValid` _returnvalue
    (:`Is Valid`
      (`self.EnableInput` _returnvalue self))))

(fn `EndScreenMode`
  (bind _returnvalue (`|CreateWidget` "/Game/UI/UI_EndScreen.UI_EndScreen_C"))
  (set `self.EndScreenWidgetRef` _returnvalue)
  (`UserWidget.AddToViewport` (`self.EndScreenWidgetRef`) 0)
  (`WidgetBlueprintLibrary.SetInputMode_UIOnlyEx` self (`/Game/UI/UI_CustomButton.Button_0` (`/Game/UI/UI_EndScreen.MainMenuButton` (`self.EndScreenWidgetRef`))))
  (set `self.GameState` "NewEnumerator2"))

(fn `GameplaySceneMode`
  (bind _returnvalue (`GameplayStatics.GetPlayerPawn` 0))
  (`|ExecutionSequence`
    (:`then_0`
      (`/Engine/EditorBlueprintResources/StandardMacros.IsValid` (`self.DialogWidgetRef`)
        (:`Is Valid`
          (`Widget.RemoveFromParent` (`self.DialogWidgetRef`)))))
    (:`then_1`
      (`/Engine/EditorBlueprintResources/StandardMacros.IsValid` (`self.MainMenuWidgetRef`)
        (:`Is Valid`
          (`Widget.RemoveFromParent` (`self.MainMenuWidgetRef`)))))
    (:`then_2`
      (`/Engine/EditorBlueprintResources/StandardMacros.IsValid` _returnvalue
        (:`Is Valid`
          (`self.DisableInput` _returnvalue null)
          (`WidgetBlueprintLibrary.SetInputMode_GameOnly` self)
          (set `self.GameState` "NewEnumerator5"))))))

(fn `Init`
  (params (NextLevel :type Name) (CurLevel :type Name) (isStreamingEnabled :type Boolean))
  (set `self.NextLevel` NextLevel)
  (set `self.CurLevel` CurLevel)
  (set `self.isStreamingEnabled` isStreamingEnabled))

(fn `LoseScreenMode`
  (bind _returnvalue (`|CreateWidget` "/Game/UI/UI_LoseScreen.UI_LoseScreen_C"))
  (set `self.LoseScreenWidgetRef` _returnvalue)
  (`UserWidget.AddToViewport` (`self.LoseScreenWidgetRef`) 0)
  (`WidgetBlueprintLibrary.SetInputMode_UIOnlyEx` self (`/Game/UI/UI_CustomButton.Button_0` (`/Game/UI/UI_LoseScreen.Restart` (`self.LoseScreenWidgetRef`))))
  (set `self.GameState` "NewEnumerator2"))

(fn `MainMenuMode`
  (bind _returnvalue (`|CreateWidget` "/Game/UI/Widget_TestMainMenu.Widget_TestMainMenu_C"))
  (bind _output_get (set `self.MainMenuWidgetRef` _returnvalue))
  (`UserWidget.AddToViewport` _output_get 0)
  (`WidgetBlueprintLibrary.SetInputMode_UIOnlyEx` self (`/Game/UI/UI_CustomButton.Button_0` (`/Game/UI/Widget_TestMainMenu.NewGame` (`self.MainMenuWidgetRef`))))
  (set `self.GameState` "NewEnumerator2"))

(fn `PlayCutscene(F)`
  (params (Cutscene :type "/Game/BP/Testing/Cutscene_Struct Structure"))
  (bind _returnvalue (`GameplayStatics.GetPlayerPawn` 0))
  (`|ExecutionSequence`
    (:`then_0`
      (`/Engine/EditorBlueprintResources/StandardMacros.IsValid` _returnvalue
        (:`Is Valid`
          (`self.DisableInput` _returnvalue null))))
    (:`then_1`
      (bind _returnvalue_2 (`|CreateWidget` "/Game/UI/CutsceneWidgetTest.CutsceneWidgetTest_C" null (`.Frames_5_E74326014532F3E486630C99C358692B` (break `/Game/BP/Testing/Cutscene_Struct` Cutscene))))
      (bind _output_get (set `self.CutsceneWidget` _returnvalue_2))
      (`UserWidget.AddToViewport` _output_get 0))))

(fn `UserConstructionScript`)