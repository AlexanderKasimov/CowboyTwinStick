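; Base player pawn for a 2D Paper2D twin-stick shooter, playing a cowboy that moves in the XZ plane and shoots where it aims.
; Tick applies swept movement, quantizes aim into eight directions for flipbook selection, and fires unsnapped projectiles.
; Timers repeat shots at FireRate, delaying restarts so re-aiming cannot beat the cooldown.
; HandleDeath plays a cause-specific death flipbook, then restarts the level and clears projectiles when it finishes.
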(event `self.ReceiveBeginPlay`
  (set `self.LastFireTime` (/ -1.0 (`self.FireRate`))))

(event `/Game/BP/IDamagable.HandleDeath`
  (params (DeathCause :type "/Game/BP/Enum_DeathCause Enum" :default "NewEnumerator0"))
  (set `self.DeathCause` DeathCause)
  (`self.StopFire`)
  (set `self.State` "NewEnumerator4")
  (`PaperFlipbookComponent.SetFlipbook` (`self.PaperFlipbook`) (`self.GetAnimation`))
  (`PaperFlipbookComponent.SetLooping` (`self.PaperFlipbook`) false)
  (`PaperFlipbookComponent.PlayFromStart` (`self.PaperFlipbook`)))

(event `self.ReceiveTick`
  (params (DeltaSeconds :type "Float (single-precision)"))
  (bind _returnvalue (`self.GetInputAxisValue`))
  (bind _returnvalue_2 (`self.GetInputAxisValue`))
  (switch `/Game/BP/Enum_AiStates` (`self.State`)
    (:`NewEnumerator1`
      (`|ExecutionSequence`
        (:`then_0`
          (set `self.MovingInputDirection` (`KismetMathLibrary.Normal` (`KismetMathLibrary.MakeVector` (`self.GetInputAxisValue`) 0.0 (`self.GetInputAxisValue`))))
          (`self.K2_SetActorLocation` (+ (`self.K2_GetActorLocation`) (* (`self.MovingInputDirection`) (`self.Speed`))) true)
          (if (or (> (`KismetMathLibrary.Abs` _returnvalue) 0.0) (> (`KismetMathLibrary.Abs` _returnvalue_2) 0.0))
            (`|ExecutionSequence`
              (:`then_0`
                (set `self.ShootInputDirection` (`KismetMathLibrary.Normal` (`KismetMathLibrary.MakeVector` _returnvalue_2 0.0 _returnvalue)))
                (bind _quarter (`self.GetQuarter` (`self.ShootInputDirection`)))
                (set `self.ShootQuarter` _quarter))
              (:`then_1`
                (`KismetSystemLibrary.PrintString` (`KismetStringLibrary.Conv_IntToString` (`self.ShootQuarter`)) (`self.DrawDebug`) false (struct :`G` 0.66 :`B` 1.0 :`A` 1.0) 0.0)
                (`|ExecutionSequence`
                  (:`then_0`
                    (bind _direction (`self.GetDirection` (`self.ShootQuarter`) (`self.ShootInputDirection`)))
                    (set `self.ShootingDirection` _direction))
                  (:`then_1`
                    (if (not (`self.isFiring`))
                      (`self.StartStartFire`))))))
            (else
              (`self.StopFire`))))
        (:`then_1`
          (`PaperFlipbookComponent.SetFlipbook` (`self.PaperFlipbook`) (`self.GetAnimation`))
          (`PaperFlipbookComponent.SetLooping` (`self.PaperFlipbook`) true))))))

(event `self.PaperFlipbook.OnFinishedPlaying`
  (switch `/Game/BP/Enum_AiStates` (`self.State`)
    (:`NewEnumerator4`
      (`self.DetachFromControllerPendingDestroy`)
      (`|ExecutionSequence`
        (:`then_0`
          (bind _asbp_base_player_controller (cast `/Game/BP/BP_BasePlayerController` (`GameplayStatics.GetPlayerController` 0)))
          (`/Game/BP/BP_BasePlayerController.Restart Level` _asbp_base_player_controller)
          (`self.K2_DestroyActor`))
        (:`then_1`
          (bind _outactors (`GameplayStatics.GetAllActorsOfClass` "/Game/BP/BP_BaseProjectile.BP_BaseProjectile_C"))
          (for _array_element _outactors
            (`self.K2_DestroyActor` _array_element)))))))

(fn `Fire`
  (`|SpawnActorFromClass` "/Game/BP/BP_ProjectileCowboy.BP_ProjectileCowboy_C" (`KismetMathLibrary.Conv_VectorToTransform` (+ (`self.K2_GetActorLocation`) (* (`self.ShootInputDirection`) 15.0))) "AlwaysSpawn" "OverrideRootScale" null (`self.ShootInputDirection`) 3.0 null)
  (set `self.LastFireTime` (`GameplayStatics.GetTimeSeconds`)))

(fn `GetAnimation`
  (returns (Flipbook :type "PaperFlipbook Object Reference"))
  (locals (RunUp :type "PaperFlipbook Object Reference" :default "PaperFlipbook'/Game/Sprites/CowboyRun/CowboyRunUp/FB_CowboyRunUp.FB_CowboyRunUp'") (FacingDirection :type "/Game/BP/Enum_AIFacingDirection Enum" :default "NewEnumerator1"))
  (switch `/Game/BP/Enum_AiStates` (`self.State`)
    (:`NewEnumerator1`
      (if (> (`KismetMathLibrary.VSize` (`self.MovingInputDirection`)) 0.0)
        (return (select `/Game/BP/Enum_Direction` (`self.ShootingDirection`) :`NewEnumerator0` "/Game/Sprites/CowboyRun/CowboyRunDown/FB_CowboyRunDown.FB_CowboyRunDown" :`NewEnumerator1` (`local.RunUp`) :`NewEnumerator2` "/Game/Sprites/CowboyRun/CowboyRunUpRight/FB_CowboyRunUpRight.FB_CowboyRunUpRight" :`NewEnumerator3` "/Game/Sprites/CowboyRun/CowboyRunRight/FB_CowboyRunRight.FB_CowboyRunRight" :`NewEnumerator4` "/Game/Sprites/CowboyRun/CowboyRunDownRight/FB_CowboyRunDownRight.FB_CowboyRunDownRight" :`NewEnumerator5` "/Game/Sprites/CowboyRun/CowboyRunDown/FB_CowboyRunDown.FB_CowboyRunDown" :`NewEnumerator6` "/Game/Sprites/CowboyRun/CowboyRunDownLeft/FB_CowboyRunDownLeft.FB_CowboyRunDownLeft" :`NewEnumerator7` "/Game/Sprites/CowboyRun/CowboyRunLeft/FB_CowboyRunLeft.FB_CowboyRunLeft" :`NewEnumerator8` "/Game/Sprites/CowboyRun/CowboyRunUpLeft/FB_CowboyRunUpLeft.FB_CowboyRunUpLeft"))
        (else
          (return (select `/Game/BP/Enum_Direction` (`self.ShootingDirection`) :`NewEnumerator0` "/Game/Sprites/CowboyIdle/CowboyIdleDown/FB_CowboyIdleDown_Flipbook.FB_CowboyIdleDown_Flipbook" :`NewEnumerator1` "/Game/Sprites/CowboyIdle/CowboyIdleUp/FB_CowboyIdleUp_Flipbook.FB_CowboyIdleUp_Flipbook" :`NewEnumerator2` "/Game/Sprites/CowboyIdle/CowboyIdleUpRight/FB_CowboyIdleUpRight_Flipbook.FB_CowboyIdleUpRight_Flipbook" :`NewEnumerator3` "/Game/Sprites/CowboyIdle/CowboyIdleRight/FB_CowboyIdleRight_Flipbook.FB_CowboyIdleRight_Flipbook" :`NewEnumerator4` "/Game/Sprites/CowboyIdle/CowboyIdleDownRight/FB_CowboyIdleDownRight_Flipbook.FB_CowboyIdleDownRight_Flipbook" :`NewEnumerator5` "/Game/Sprites/CowboyIdle/CowboyIdleDown/FB_CowboyIdleDown_Flipbook.FB_CowboyIdleDown_Flipbook" :`NewEnumerator6` "/Game/Sprites/CowboyIdle/CowboyIdleDownLeft/FB_CowboyIdleDownLeft_Flipbook.FB_CowboyIdleDownLeft_Flipbook" :`NewEnumerator7` "/Game/Sprites/CowboyIdle/CowboyIdleLeft/FB_CowboyIdleLeft_Flipbook.FB_CowboyIdleLeft_Flipbook" :`NewEnumerator8` "/Game/Sprites/CowboyIdle/CowboyIdleUpLeft/FB_CowboyIdleUpLeft_Flipbook.FB_CowboyIdleUpLeft_Flipbook" :!type "PaperFlipbook Object Reference")))))
    (:`NewEnumerator4`
      (`|ExecutionSequence`
        (:`then_0`
          (switch `/Game/BP/Enum_Direction` (`self.ShootingDirection`)
            (:`NewEnumerator1`
              (set `local.FacingDirection` "NewEnumerator1" :!label _label))
            (:`NewEnumerator2`
              (goto _label))
            (:`NewEnumerator3`
              (goto _label))
            (:`NewEnumerator4`
              (goto _label))
            (:`NewEnumerator5`
              (set `local.FacingDirection` "NewEnumerator0" :!label _label_2))
            (:`NewEnumerator6`
              (goto _label_2))
            (:`NewEnumerator7`
              (goto _label_2))
            (:`NewEnumerator8`
              (goto _label_2))))
        (:`then_1`
          (switch `/Game/BP/Enum_AIFacingDirection` (`local.FacingDirection`)
            (:`NewEnumerator0`
              (return (select `/Game/BP/Enum_DeathCause` (`self.DeathCause`) :`NewEnumerator0` "/Game/Sprites/CowboyDeath/SwordDeathLeft/FB_SwordDeathLeft.FB_SwordDeathLeft" :`NewEnumerator1` "/Game/Sprites/CowboyDeath/SwordDeathLeft/FB_SwordDeathLeft.FB_SwordDeathLeft" :`NewEnumerator2` "/Game/Sprites/CowboyDeath/FireballDeathLeft/FB_FireballDeathLeft.FB_FireballDeathLeft" :`NewEnumerator3` "/Game/Sprites/CowboyDeath/BossDemonDeathLeft/FB_BossDemonDeathLeft.FB_BossDemonDeathLeft" :!type "PaperFlipbook Object Reference")))
            (:`NewEnumerator1`
              (return (select `/Game/BP/Enum_DeathCause` (`self.DeathCause`) :`NewEnumerator0` "/Game/Sprites/CowboyDeath/SwordDeathRight/FB_SwordDeathRight.FB_SwordDeathRight" :`NewEnumerator1` "/Game/Sprites/CowboyDeath/SwordDeathRight/FB_SwordDeathRight.FB_SwordDeathRight" :`NewEnumerator2` "/Game/Sprites/CowboyDeath/FireballDeathRight/FB_FireballDeathRight.FB_FireballDeathRight" :`NewEnumerator3` "/Game/Sprites/CowboyDeath/BossDemonDeathRight/FB_BossDemonDeathRight.FB_BossDemonDeathRight" :!type "PaperFlipbook Object Reference")))))))))

(fn `GetDirection`
  (params (Quarter :type Integer) (InputVector :type "Vector Structure"))
  (returns (Direction :type "/Game/BP/Enum_Direction Enum"))
  (locals (LocalInputVector :type "Vector Structure"))
  (set `local.LocalInputVector` InputVector)
  (switch `int` Quarter
    (:`1`
      (if (`KismetMathLibrary.InRange_FloatFloat` (`KismetMathLibrary.DegAcos` (`KismetMathLibrary.Dot_VectorVector` (`local.LocalInputVector`) (0.0 0.0 1.0))) 0.0 15.0)
        (return "NewEnumerator1")
        (elif (`KismetMathLibrary.InRange_FloatFloat` (`KismetMathLibrary.DegAcos` (`KismetMathLibrary.Dot_VectorVector` (`local.LocalInputVector`) (0.0 0.0 1.0))) 15.0 75.0 false)
          (return "NewEnumerator2")
          (else
            (return "NewEnumerator3")))))
    (:`2`
      (if (`KismetMathLibrary.InRange_FloatFloat` (`KismetMathLibrary.DegAcos` (`KismetMathLibrary.Dot_VectorVector` (`local.LocalInputVector`) (0.0 0.0 1.0))) 0.0 15.0)
        (return "NewEnumerator1")
        (elif (`KismetMathLibrary.InRange_FloatFloat` (`KismetMathLibrary.DegAcos` (`KismetMathLibrary.Dot_VectorVector` (`local.LocalInputVector`) (0.0 0.0 1.0))) 15.0 75.0 false)
          (return "NewEnumerator8")
          (else
            (return "NewEnumerator7")))))
    (:`3`
      (if (`KismetMathLibrary.InRange_FloatFloat` (`KismetMathLibrary.DegAcos` (`KismetMathLibrary.Dot_VectorVector` (`local.LocalInputVector`) (0.0 0.0 -1.0))) 0.0 15.0)
        (return "NewEnumerator5")
        (elif (`KismetMathLibrary.InRange_FloatFloat` (`KismetMathLibrary.DegAcos` (`KismetMathLibrary.Dot_VectorVector` (`local.LocalInputVector`) (0.0 0.0 -1.0))) 15.0 75.0 false)
          (return "NewEnumerator6")
          (else
            (return "NewEnumerator7")))))
    (:`4`
      (if (`KismetMathLibrary.InRange_FloatFloat` (`KismetMathLibrary.DegAcos` (`KismetMathLibrary.Dot_VectorVector` (`local.LocalInputVector`) (0.0 0.0 -1.0))) 0.0 15.0)
        (return "NewEnumerator5")
        (elif (`KismetMathLibrary.InRange_FloatFloat` (`KismetMathLibrary.DegAcos` (`KismetMathLibrary.Dot_VectorVector` (`local.LocalInputVector`) (0.0 0.0 -1.0))) 15.0 75.0 false)
          (return "NewEnumerator4")
          (else
            (return "NewEnumerator3")))))))

(fn `GetQuarter`
  (params (InputVector :type "Vector Structure"))
  (returns (Quarter :type Integer))
  (locals (LocalInputVector :type "Vector Structure"))
  (set `local.LocalInputVector` InputVector)
  (if (and (>= (.x (`local.LocalInputVector`)) 0.0) (>= (.z (`local.LocalInputVector`)) 0.0))
    (return 1)
    (elif (and (<= (.x (`local.LocalInputVector`)) 0.0) (>= (.z (`local.LocalInputVector`)) 0.0))
      (return 2)
      (elif (and (<= (.x (`local.LocalInputVector`)) 0.0) (<= (.z (`local.LocalInputVector`)) 0.0))
        (return 3)
        (elif (and (>= (.x (`local.LocalInputVector`)) 0.0) (<= (.z (`local.LocalInputVector`)) 0.0))
          (return 4))))))

(fn `StartFire`
  (`self.Fire`)
  (bind _returnvalue (`KismetSystemLibrary.K2_SetTimer` null "Fire" (/ 1.0 (`self.FireRate`)) true))
  (set `self.FireTimerHandle` _returnvalue))

(fn `StartStartFire`
  (set `self.isFiring` true)
  (bind _returnvalue (`KismetSystemLibrary.K2_SetTimer` null "StartFire" (`KismetMathLibrary.FMax` (- (+ (`self.LastFireTime`) (/ 1.0 (`self.FireRate`))) (`GameplayStatics.GetTimeSeconds`)) 1e-05)))
  (set `self.StartStartFireTimerHandle` _returnvalue))

(fn `StopFire`
  (`KismetSystemLibrary.K2_ClearAndInvalidateTimerHandle` (`self.StartStartFireTimerHandle`))
  (`KismetSystemLibrary.K2_ClearAndInvalidateTimerHandle` (`self.FireTimerHandle`))
  (set `self.isFiring` false))

(fn `Teleport`
  (params (Location :type "Vector Structure"))
  (`self.K2_SetActorLocation` Location))

(fn `UserConstructionScript`)