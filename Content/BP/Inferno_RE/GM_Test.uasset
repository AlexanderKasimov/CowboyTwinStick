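; Test game mode that runs progression through streamed levels and owns the gameplay UI widget with its screen fades.
; Level load and transition events drive the widget fade and toggle pawn movement.
; Fade events swap streaming levels, calling a clear-level dispatcher and resetting kills, or activate every TestSpawner.
; Kills are counted against the LevelInfo enemy quota, which unlocks the current level's transition once met.
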(event `self.ReceiveBeginPlay`
  (bind _returnvalue (`|CreateWidget` "/Game/UI/Inferno_RE/UI_Gameplay.UI_Gameplay_C"))
  (bind _output_get (set `self.GameplayWidget` _returnvalue))
  (`UserWidget.AddToViewport` _output_get 0))

(event `/Game/BP/Inferno_RE/Interfaces/LevelManagement.LevelLoaded`
  (params (LevelInfo :type "/Game/BP/Inferno_RE/Structs/LevelInfo Structure"))
  (set `self.LevelInfo` LevelInfo)
  (`/Game/BP/Inferno_RE/Interfaces/UIManagement.FadeOut` (`self.GameplayWidget`))
  (`KismetSystemLibrary.Delay` 0.5)
  (message `/Game/BP/Inferno_RE/Interfaces/GameplayManagement.EnableMovement` (`GameplayStatics.GetPlayerPawn` 0)))

(event `/Game/BP/Inferno_RE/Interfaces/LevelManagement.NextLevel`
  (`/Game/BP/Inferno_RE/Interfaces/UIManagement.FadeIn` (`self.GameplayWidget`))
  (message `/Game/BP/Inferno_RE/Interfaces/GameplayManagement.DisableMovement` (`GameplayStatics.GetPlayerPawn` 0)))

(event `/Game/BP/Inferno_RE/Interfaces/UIManagement.FadeIn`
  (`|ExecutionSequence`
    (:`then_0`
      (`GameplayStatics.UnloadStreamLevel` (`.LevelName_7_14EEB359465E77D09AD631B1E2FE198E` (break `/Game/BP/Inferno_RE/Structs/LevelInfo` (`self.LevelInfo`))))
      (`self.ClearLevel`)
      (`GameplayStatics.LoadStreamLevel` (`.NextLevelName_5_268CEDD74402361ACFBD3FA7E32312CA` (break `/Game/BP/Inferno_RE/Structs/LevelInfo` (`self.LevelInfo`))) true))
    (:`then_2`
      (set `self.EnemiesKilled` 0))))

(event `/Game/BP/Inferno_RE/Interfaces/UIManagement.FadeOut`
  (`|ExecutionSequence`
    (:`then_0`
      ;[1 1 1] Лучше делегат -> активировать всех противников
      (bind _outactors (`GameplayStatics.GetAllActorsOfClass` "/Game/BP/Inferno_RE/TestSpawner.TestSpawner_C"))
      (for _array_element _outactors
        (`/Game/BP/Inferno_RE/TestSpawner.ActivateSpawners` _array_element)))))

(event `/Game/BP/Inferno_RE/Interfaces/GameplayManagement.EnemyKilled`
  (`/Engine/EditorBlueprintResources/StandardMacros.IncrementInt` (`self.EnemiesKilled`)
    (:`  `
      (if (>= (`self.EnemiesKilled`) (`.EnemiesCount_2_B54E7AA34895E4BD0DCA879F00CEE780` (break `/Game/BP/Inferno_RE/Structs/LevelInfo` (`self.LevelInfo`))))
        (message `/Game/BP/Inferno_RE/Interfaces/GameplayManagement.AllowTransition` (`GameplayStatics.GetStreamingLevel` (`.LevelName_7_14EEB359465E77D09AD631B1E2FE198E` (break `/Game/BP/Inferno_RE/Structs/LevelInfo` (`self.LevelInfo`)))))))))

(fn `UserConstructionScript`)