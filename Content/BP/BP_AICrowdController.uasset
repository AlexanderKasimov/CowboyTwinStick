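; Crowd controller that starts an encounter of melee cultists and a mage when its ActivateAI event is called.
; It assigns each of the first four valid MeleeCultists a fixed, distinct attack spot and clears its cutscene mode, then activates the Mage if valid.
; Tick does nothing, and leftover debug box traces on either side of the player are never run.
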(event `self.ReceiveBeginPlay`)

(event `ActivateAI`
  (`self.UpdateCultistsTargetSpots`)
  (`self.ActivateMage`))

(event `self.ReceiveTick`
  (params (DeltaSeconds :type "Float (single-precision)")))

(fn `ActivateMage`
  (`/Engine/EditorBlueprintResources/StandardMacros.IsValid` (`self.Mage`)
    (:`Is Valid`
      (`/Game/BP/BP_EnemyMage.Activate` (`self.Mage`)))))

(fn `UpdateCultistsTargetSpots`
  (bind _output (`|GetArrayItem` (`self.MeleeCultists`) 2))
  (bind _output_2 (`|GetArrayItem` (`self.MeleeCultists`) 3))
  (bind _output_3 (`|GetArrayItem` (`self.MeleeCultists`)))
  (bind _output_4 (`|GetArrayItem` (`self.MeleeCultists`) 1))
  (`|ExecutionSequence`
    (:`then_0`
      (`/Engine/EditorBlueprintResources/StandardMacros.IsValid` _output_3
        (:`Is Valid`
          (`/Game/BP/BP_EnemyCultist.SetAttackSpot` _output_3 "NewEnumerator1")
          (set `/Game/BP/BP_BaseEnemy.CutsceneMode` false _output_3))))
    (:`then_1`
      (`/Engine/EditorBlueprintResources/StandardMacros.IsValid` _output_4
        (:`Is Valid`
          (`/Game/BP/BP_EnemyCultist.SetAttackSpot` _output_4 "NewEnumerator2")
          (set `/Game/BP/BP_BaseEnemy.CutsceneMode` false _output_4))))
    (:`then_2`
      (`/Engine/EditorBlueprintResources/StandardMacros.IsValid` _output
        (:`Is Valid`
          (`/Game/BP/BP_EnemyCultist.SetAttackSpot` _output "NewEnumerator5")
          (set `/Game/BP/BP_BaseEnemy.CutsceneMode` false _output))))
    (:`then_3`
      (`/Engine/EditorBlueprintResources/StandardMacros.IsValid` _output_2
        (:`Is Valid`
          (`/Game/BP/BP_EnemyCultist.SetAttackSpot` _output_2 "NewEnumerator6")
          (set `/Game/BP/BP_BaseEnemy.CutsceneMode` false _output_2))))))

(fn `UserConstructionScript`)