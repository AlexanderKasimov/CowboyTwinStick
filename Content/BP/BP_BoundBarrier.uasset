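; BP_BoundBarrier is a barrier actor drawn with a Paper2D flipbook that can be switched on and off.
; DisableBarrier turns off the flipbook's collision and hides it.
; EnableBarrier restores query-only collision and shows it again.
; The blueprint has no other active logic, so it relies on other code to call these two events.
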(event `DisableBarrier`
  (`PrimitiveComponent.SetCollisionEnabled` (`self.PaperFlipbook`) "NoCollision")
  (`SceneComponent.SetVisibility` (`self.PaperFlipbook`) false false))

(event `Enable Barrier`
  (`PrimitiveComponent.SetCollisionEnabled` (`self.PaperFlipbook`) "QueryOnly")
  (`SceneComponent.SetVisibility` (`self.PaperFlipbook`) true false))

(fn `UserConstructionScript`)