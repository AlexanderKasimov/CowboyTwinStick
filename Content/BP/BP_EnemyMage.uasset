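; Paper2D mage enemy that faces the player and repeatedly casts fireballs at them once activated out of cutscene mode.
; An Idle/Attacking/Dying state and facing direction select flipbooks, and flipbook completion drives the cast phases, projectile spawn and timed next attack.
; Its health component loses immortality once all cultist guards have died.
; Death stops the attack timer and plays a death flipbook before announcing MageDied and running parent death handling.
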(event `self.ReceiveBeginPlay`
  (`parent.ReceiveBeginPlay`))

(event `Activate`
  (set `self.CutsceneMode` false)
  (`KismetSystemLibrary.Delay` 2.0)
  (`self.Attack`))

(event `PlayAnimation`
  (params (Animation :type "PaperFlipbook Soft Object Reference") (isLooping :type Boolean) (PlayRate :type "Float (double-precision)"))
  (set `self.isLooping` isLooping)
  (bind _object (`|LoadAsset` Animation)
    (:`Completed`
      (bind _aspaper_flipbook (cast `PaperFlipbook` _object))
      (`PaperFlipbookComponent.SetFlipbook` (`self.PaperFlipbook`) _aspaper_flipbook)
      (`PaperFlipbookComponent.SetLooping` (`self.PaperFlipbook`) (`self.isLooping`))
      (`PaperFlipbookComponent.PlayFromStart` (`self.PaperFlipbook`)))))

(event `self.ReceiveTick`
  (params (DeltaSeconds :type "Float (single-precision)"))
  (bind _returnvalue (`GameplayStatics.GetPlayerPawn` 0))
  (`parent.ReceiveTick` DeltaSeconds)
  (if (not (`self.CutsceneMode`))
    (`|ExecutionSequence`
      (:`then_0`
        (`/Engine/EditorBlueprintResources/StandardMacros.IsValid` _returnvalue
          (:`Is Valid`
            (if (<= (.x (- (`self.K2_GetActorLocation` _returnvalue) (`self.K2_GetActorLocation`))) 0.0)
              (set `self.FacingDirection` "NewEnumerator0")
              (else
                (set `self.FacingDirection` "NewEnumerator1"))))))
      (:`then_1`
        (switch `/Game/BP/Enum_AiStates` (`self.State`)
          (:`NewEnumerator5`
            (bind _flipbook (`self.GetAnimation`))
            (`PaperFlipbookComponent.SetFlipbook` (`self.PaperFlipbook`) _flipbook)
            (`PaperFlipbookComponent.SetLooping` (`self.PaperFlipbook`) true)))))))

(event `/Game/BP/IAICommunication.GuardDied`
  (params (Guard :type "/Game/BP/BP_BaseEnemy Object Reference"))
  (bind _asbp_enemy_cultist (cast `/Game/BP/BP_EnemyCultist` Guard))
  (`KismetArrayLibrary.Array_RemoveItem` (`self.Guards`) _asbp_enemy_cultist)
  (if (<= (`KismetArrayLibrary.Array_Length` (`self.Guards`)) 0)
    (`/Game/BP/BP_BaseHealthComponent.SetImmortal` (`self.BP_BaseHealthComponent`) false)))

(event `self.HandleDeath`
  (params (DeathCause :type "/Game/BP/Enum_DeathCause Enum" :default "NewEnumerator0"))
  (set `self.State` "NewEnumerator4")
  (`KismetSystemLibrary.K2_ClearAndInvalidateTimerHandle` (`self.AttackTimerHandle`))
  (bind _flipbook (`self.GetAnimation`))
  (`PaperFlipbookComponent.SetFlipbook` (`self.PaperFlipbook`) _flipbook)
  (`PaperFlipbookComponent.SetLooping` (`self.PaperFlipbook`) false)
  (`PaperFlipbookComponent.PlayFromStart` (`self.PaperFlipbook`)))

(event `self.PaperFlipbook.OnFinishedPlaying`
  (bind _returnvalue (`PaperFlipbookComponent.GetFlipbook` (`self.PaperFlipbook`)))
  (if (not (`self.CutsceneMode`))
    (switch `/Game/BP/Enum_AiStates` (`self.State`)
      (:`NewEnumerator3`
        (if (or (== _returnvalue "/Game/Sprites/Mage/MageCastLeft/FB_MageCastLeft_Begin.FB_MageCastLeft_Begin") (== _returnvalue "/Game/Sprites/Mage/MageCastRight/FB_MageCastRight_Begin.FB_MageCastRight_Begin"))
          (`|ExecutionSequence`
            (:`then_0`
              (bind _flipbook (`self.GetAnimation`))
              (`PaperFlipbookComponent.SetFlipbook` (`self.PaperFlipbook`) _flipbook)
              (`PaperFlipbookComponent.PlayFromStart` (`self.PaperFlipbook`)))
            (:`then_1`
              (`self.CastFireball`)))
          (elif (or (== (`PaperFlipbookComponent.GetFlipbook` (`self.PaperFlipbook`)) "/Game/Sprites/Mage/MageCastLeft/FB_MageCastLeft_End.FB_MageCastLeft_End") (== (`PaperFlipbookComponent.GetFlipbook` (`self.PaperFlipbook`)) "/Game/Sprites/Mage/MageCastRight/FB_MageCastRight_End.FB_MageCastRight_End"))
            (set `self.State` "NewEnumerator5")
            (`PaperFlipbookComponent.PlayFromStart` (`self.PaperFlipbook`))
            (bind _returnvalue_2 (`KismetSystemLibrary.K2_SetTimer` null "Attack" 2.0))
            (set `self.AttackTimerHandle` _returnvalue_2))))
      (:`NewEnumerator4`
        (`self.MageDied`)
        (`parent.HandleDeath` "NewEnumerator0")))))

(fn `Attack`
  (set `self.State` "NewEnumerator3")
  (bind _flipbook (`self.GetAnimation`))
  (`PaperFlipbookComponent.SetFlipbook` (`self.PaperFlipbook`) _flipbook)
  (`PaperFlipbookComponent.SetLooping` (`self.PaperFlipbook`) false)
  (`PaperFlipbookComponent.PlayFromStart` (`self.PaperFlipbook`)))

(fn `CastFireball`
  (bind _returnvalue (`GameplayStatics.GetPlayerPawn` 0))
  (bind _returnvalue_2 (`KismetMathLibrary.Normal` (- (`self.K2_GetActorLocation` _returnvalue) (`self.K2_GetActorLocation`))))
  (`/Engine/EditorBlueprintResources/StandardMacros.IsValid` _returnvalue
    (:`Is Valid`
      (`|SpawnActorFromClass` "/Game/BP/BP_ProjectileFireball.BP_ProjectileFireball_C" (`KismetMathLibrary.Conv_VectorToTransform` (+ (`self.K2_GetActorLocation`) (* _returnvalue_2 16.0))) "Undefined" "OverrideRootScale" null _returnvalue_2 210.0 null))))

(fn `GetAnimation`
  (returns (Flipbook :type "PaperFlipbook Object Reference"))
  (bind _returnvalue (`PaperFlipbookComponent.GetFlipbook` (`self.PaperFlipbook`)))
  (switch `/Game/BP/Enum_AiStates` (`self.State`)
    (:`NewEnumerator5`
      (return (select `/Game/BP/Enum_AIFacingDirection` (`self.FacingDirection`) :`NewEnumerator0` "/Game/Sprites/Mage/MageIdleLeft/FB_MageIdleLeft.FB_MageIdleLeft" :`NewEnumerator1` "/Game/Sprites/Mage/MageIdleRight/FB_MageIdleRight.FB_MageIdleRight" :!type "PaperFlipbook Object Reference")))
    (:`NewEnumerator3`
      (if (or (== _returnvalue "/Game/Sprites/Mage/MageCastLeft/FB_MageCastLeft_Begin.FB_MageCastLeft_Begin") (== _returnvalue "/Game/Sprites/Mage/MageCastRight/FB_MageCastRight_Begin.FB_MageCastRight_Begin"))
        (return (select `/Game/BP/Enum_AIFacingDirection` (`self.FacingDirection`) :`NewEnumerator0` "/Game/Sprites/Mage/MageCastLeft/FB_MageCastLeft_End.FB_MageCastLeft_End" :`NewEnumerator1` "/Game/Sprites/Mage/MageCastRight/FB_MageCastRight_End.FB_MageCastRight_End" :!type "PaperFlipbook Object Reference"))
        (else
          (return (select `/Game/BP/Enum_AIFacingDirection` (`self.FacingDirection`) :`NewEnumerator0` "/Game/Sprites/Mage/MageCastLeft/FB_MageCastLeft_Begin.FB_MageCastLeft_Begin" :`NewEnumerator1` "/Game/Sprites/Mage/MageCastRight/FB_MageCastRight_Begin.FB_MageCastRight_Begin" :!type "PaperFlipbook Object Reference")))))
    (:`NewEnumerator4`
      (return (select `/Game/BP/Enum_AIFacingDirection` (`self.FacingDirection`) :`NewEnumerator0` "/Game/Sprites/Mage/MageDeath/FB_MageDeath.FB_MageDeath" :`NewEnumerator1` "/Game/Sprites/Mage/MageDeathRight/FB_MageDeathRight.FB_MageDeathRight" :!type "PaperFlipbook Object Reference")))))

(fn `UserConstructionScript`
  (`parent.UserConstructionScript`))