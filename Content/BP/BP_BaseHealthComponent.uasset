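; Base health component that tracks hit points, death state and immortality for its owning actor.
; BeginPlay fills current HP from max HP, and HandleDamage subtracts damage and stores the death cause.
; At zero HP or below it flags death and passes the cause to the owner through HandleDeathMessage.
; While immortality, toggled by SetImmortal, is on, damage is ignored and a taunt string is printed.
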(event `self.ReceiveBeginPlay`
  (`self.InitHealth`))

(event `/Game/BP/IDamagable.HandleDamage`
  (params (Damage :type "Float (single-precision)") (DeathCause :type "/Game/BP/Enum_DeathCause Enum" :default "NewEnumerator0"))
  (if (not (`self.isImmortal`))
    (set `self.DeathCause` DeathCause)
    (bind _output_get (set `self.CurHP` (- (`self.CurHP`) Damage)))
    (if (<= _output_get 0.0)
      (set `self.isDead` true)
      (message `/Game/BP/IDamagable.HandleDeath` (`self.GetOwner`) (`self.DeathCause`)))
    (else
      (`KismetSystemLibrary.PrintString` "HAHAHA! I'm IMMORTAL!!!"))))

(event `/Game/BP/IDamagable.SetImmortal`
  (params (NewValue :type Boolean))
  (set `self.isImmortal` NewValue))

(fn `InitHealth`
  (set `self.CurHP` (`self.MaxHP`)))